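; BP_DialogueComponent steps through data-table-driven dialogue each time Interact is called.
; The first line creates a WB_Dialogue widget, and Update rows refresh it until EndDialogue removes it and resets the row name.
; Each row chains to the next row and table and sets the flow flags, with AboutToEnd incrementing NoteNumber on the following advance.
; Interacting while text is only partly displayed reveals the full line instead of advancing.
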(event `/Game/DialogueBPs/BP_Interact.Interact`
  (params (PlayerRef :type "/Game/FirstPerson/Blueprints/BP_FirstPersonCharacter Object Reference"))
  (bind _dialoguewidget (`self.DialogueWidget`))
  (if (`KismetStringLibrary.EqualEqual_StrStr` (`/Game/DialogueBPs/WB_Dialogue.SFullText` _dialoguewidget) (`/Game/DialogueBPs/WB_Dialogue.SDisplayText` _dialoguewidget))
    (if (`self.bAboutToEnd`)
      (set `self.NoteNumber` (+ 1 (`self.NoteNumber`))))
    (if (`self.bEndDialogue`)
      (`Widget.RemoveFromParent` (`self.DialogueWidget`))
      (set `self.bEndDialogue` false)
      (set `self.DialogueWidget` null)
      (set `self.bUpdate` false)
      (set `self.Row Name` "1")
      (elif (`self.bUpdate`)
        (bind _returnvalue (`|GetDataTableRow` (`self.Data Table`) (`self.Row Name`))
          (:`then`
            (bind (_nrow _sdialoguetext _datatableref _benddialogue _bupdate _babouttoend) (break `/Game/DialogueBPs/DialogueStructure` _returnvalue))
            (`/Game/DialogueBPs/WB_Dialogue.Update Dialogue` (`self.DialogueWidget`) _sdialoguetext)
            (set `self.Row Name` _nrow)
            (set `self.Data Table` _datatableref)
            (set `self.bEndDialogue` _benddialogue)
            (set `self.bUpdate` _bupdate)
            (set `self.bAboutToEnd` _babouttoend)))
        (else
          (bind _returnvalue_2 (`|GetDataTableRow` (`self.Data Table`) (`self.Row Name`))
            (:`then`
              (bind (_nrow_2 _sdialoguetext_2 _datatableref_2 _benddialogue_2 _bupdate_2 _babouttoend_2) (break `/Game/DialogueBPs/DialogueStructure` _returnvalue_2))
              (bind _returnvalue_3 (`|CreateWidget` "/Game/DialogueBPs/WB_Dialogue.WB_Dialogue_C" null _sdialoguetext_2))
              (set `self.DialogueWidget` _returnvalue_3)
              (set `self.Row Name` _nrow_2)
              (set `self.Data Table` _datatableref_2)
              (set `self.bEndDialogue` _benddialogue_2)
              (`UserWidget.AddToViewport` _returnvalue_3 0)
              (set `self.bUpdate` _bupdate_2)
              (set `self.bAboutToEnd` _babouttoend_2))))))
    (else
      (set `/Game/DialogueBPs/WB_Dialogue.SDisplayText` (`/Game/DialogueBPs/WB_Dialogue.SFullText` _dialoguewidget) _dialoguewidget))))